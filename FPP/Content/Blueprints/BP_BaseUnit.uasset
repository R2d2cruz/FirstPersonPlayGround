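; Base character Blueprint for a melee combat unit with movement, aiming, team affiliation, health and death.
; Combo, secondary and held charged attacks play montages and set an index that selects damage and trace socket.
; HitDetect sphere-traces at that socket and damages BPI_Unit actors on other teams.
; Received damage picks front or back reaction or death montages by dot product, locking attacks and movement; death also disables capsule collision and gravity.
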(event EventOnHitReactionEnd
  (Variables|Default|SetGettingHit false)
  (Variables|Default|SetIsAttacking false))

(event Collision|EventActorBeginOverlap
  (params (OtherActor :type Actor%20Object%20Reference)))

(event EventTick
  (params (DeltaSeconds :type Float%20%28single-precision%29)))

(event EventBeginPlay
  (Variables|Default|SetCanCombo false)
  (Variables|Default|SetIsAttacking false)
  (Variables|Default|SetSpeedMultiplier 0.5)
  (Variables|Default|SetHealt 1e+02)
  (Variables|Default|SetDamages (Utilities|Array|MakeArray 1e+01 1e+01 15.0 35.0)))

(event Game|Damage|EventAnyDamage
  (params (Damage :type Float%20%28single-precision%29) (DamageType :type Damage%20Type%20Object%20Reference) (InstigatedBy :type Controller%20Object%20Reference) (DamageCauser :type Actor%20Object%20Reference))
  (CallFunction|HitReaction DamageCauser Damage))

(event EventEnableCombo
  (Variables|Default|SetCanCombo true))

(fn ConstructionScript)

(fn Move
  (params (x :type Float%20%28double-precision%29) (y :type Float%20%28double-precision%29))
  (bind _speedmultiplier (Variables|Default|GetSpeedMultiplier))
  ;[0.15 0.15 0.15 0.5] Move Function
  (if (not (Variables|Default|GetIsAttacking))
    (Pawn|Input|AddMovementInput (Transformation|GetActorForwardVector) (* x _speedmultiplier) false)
    (Pawn|Input|AddMovementInput (Transformation|GetActorRightVector) (* y _speedmultiplier) false)))

(fn Aim
  (params (Yaw :type Float%20%28double-precision%29) (Aim :type Float%20%28double-precision%29))
  ;[0.15 0.15 0.15 0.5] Aim Function
  (Pawn|Input|AddControllerYawInput Yaw)
  (Pawn|Input|AddControllerPitchInput Aim))

(fn Attack2
  (if (not (Variables|Default|GetIsAttacking))
    (Variables|Default|SetIsAttacking true)
    (Variables|Default|SetAttackIndex 2)
    (Animation|PlayAnimMontage "/Game/Characters/Mannequins/Anims/Unarmed/Attack/MM_Attack_03_Montage.MM_Attack_03_Montage" 1.0 "None")))

(fn Attack1
  (if (not (Variables|Default|GetIsHolding))
    (if (Variables|Default|GetIsAttacking)
      (if (Variables|Default|GetCanCombo)
        (Variables|Default|SetAttackIndex 1)
        (Variables|Default|SetCanCombo false)
        (Variables|Default|SetIsAttacking true)
        (Animation|PlayAnimMontage "/Game/Characters/Mannequins/Anims/Unarmed/Attack/MM_Attack_02_Montage.MM_Attack_02_Montage" 1.0 "None")
        (else
          (return)))
      (else
        (Variables|Default|SetAttackIndex 0)
        (Variables|Default|SetIsAttacking true)
        (Animation|PlayAnimMontage "/Game/Characters/Mannequins/Anims/Unarmed/Attack/MM_Attack_01_Montage.MM_Attack_01_Montage" 1.0 "None")))
    (else
      (return))))

(fn HoldAttack
  (params (ElapsedTime :type Float%20%28double-precision%29))
  (if (and (not (Variables|Default|GetIsAttacking)) (>= ElapsedTime 0.2))
    (Variables|Default|SetIsAttacking true)
    (Variables|Default|SetAttackIndex 3)
    (Animation|PlayAnimMontage "/Game/Characters/Mannequins/Anims/Unarmed/Attack/MM_ChargedAttack_Montage.MM_ChargedAttack_Montage" 1.0 "None")))

(fn Hit
  (params (OtherActor :type Actor%20Object%20Reference))
  (if (and (!= OtherActor self) (Utilities|DoesObjectImplementInterface OtherActor "/Game/Blueprints/BPI_Unit.BPI_Unit_C"))
    (bind _team (Class|BPIUnit|GetTeam(Message) OtherActor))
    (if (!= _team (Variables|Default|GetTeam))
      (Game|Damage|ApplyDamage OtherActor (Utilities|Array|Get(acopy) (Variables|Default|GetDamages) (Variables|Default|GetAttackIndex)) 0 self "/Script/Engine.DamageType"))))

(fn HitDetect
  (bind _mesh (Variables|Character|GetMesh))
  (bind _socketsnames (LocalVariables|GetSocketsNames))
  (bind _attackindex (Variables|Default|GetAttackIndex))
  (bind _output (Utilities|Array|Get(acopy) _socketsnames _attackindex))
  (bind _returnvalue (Transformation|GetSocketLocation _mesh _output))
  (bind _outhit (Collision|SphereTraceForObjects _returnvalue _returnvalue 5e+01 (Utilities|Array|MakeArray "ObjectTypeQuery3") false 0 "ForDuration"))
  (CallFunction|Hit (.HitActor (Collision|BreakHitResult _outhit))))

(fn HitReaction
  (params (DamageCauser :type Actor%20Object%20Reference) (BaseDamage :type Float%20%28double-precision%29))
  (if (not (Variables|Default|GetGettingHit))
    (Variables|Default|SetGettingHit true)
    (Variables|Default|SetCanCombo false)
    (Variables|Default|SetIsAttacking true)
    (bind _output_get (Variables|Default|SetHealt (- (Variables|Default|GetHealt) BaseDamage)))
    (Development|PrintString (Utilities|String|ToString(Float) _output_get))
    (if (> (Math|Vector|DotProduct (Math|Vector|Normalize (- (Transformation|GetActorLocation DamageCauser) (Transformation|GetActorLocation))) (Transformation|GetActorForwardVector)) 0.0)
      (LocalVariables|SetPositionIndex 1)
      (else
        (LocalVariables|SetPositionIndex 0)))
    (if (> (Variables|Default|GetHealt) 0.0)
      (Animation|PlayAnimMontage (Utilities|Array|Get(acopy) (Utilities|Array|MakeArray "/Game/Blueprints/Anim/Mixamo/HitReaction/RMM_Standing_React_Large_From_Back_Montage.RMM_Standing_React_Large_From_Back_Montage" "/Game/Blueprints/Anim/Mixamo/HitReaction/RMM_Standing_React_Large_From_Front_Montage.RMM_Standing_React_Large_From_Front_Montage") (LocalVariables|GetPositionIndex)) 1.0 "None")
      (else
        (CallFunction|Die (LocalVariables|GetPositionIndex) 0.0)))))

(fn Die
  (params (Position%20Index :type Integer) (ExtraTime :type Float%20%28double-precision%29))
  (Collision|SetCollisionEnabled (Variables|Collision|GetCapsuleComponent) "NoCollision")
  (Variables|/Script/Engine.CharacterMovementComponent|SetGravityScale (Variables|Character|GetCharacterMovement) 0.0)
  (bind _returnvalue (Animation|PlayAnimMontage (Utilities|Array|Get(acopy) (Utilities|Array|MakeArray "/Game/Blueprints/Anim/Mixamo/Death/RMM_Standing_Death_Backward_01_Montage.RMM_Standing_Death_Backward_01_Montage" "/Game/Blueprints/Anim/Mixamo/Death/RMM_Standing_Death_Forward_01_Montage.RMM_Standing_Death_Forward_01_Montage") Position%20Index) 1.0 "None"))
  (Utilities|Time|SetTimerbyEvent (EventDispatchers|CreateEvent :!event OnDieMontageFinish) (+ _returnvalue ExtraTime)))

(fn OnDieMontageFinish)

(fn GetAttackIndex
  (return (Variables|Default|GetAttackIndex)))

(fn GetIsAttacking
  (return (Variables|Default|GetIsAttacking)))

(fn GetTeam
  (return (Variables|Default|GetTeam)))

(fn OnAttackEnd
  (Variables|Default|SetIsAttacking false)
  (return))