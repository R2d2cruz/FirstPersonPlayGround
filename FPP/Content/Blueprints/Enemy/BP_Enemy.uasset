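; BP_Enemy is an enemy actor Blueprint that builds on a parent class and assigns itself to team 1 on BeginPlay.
; Its Die override calls the parent with the given position index but forces the extra time to zero, then makes its controller unpossess it.
; Tick and the construction script only forward to the parent, and the overlap event is disabled.
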(event EventBeginPlay
  (|CallParentFunction)
  (Variables|Default|SetTeam 1))

(event Collision|EventActorBeginOverlap
  (params (OtherActor :type Actor%20Object%20Reference))
  (|CallParentFunction OtherActor) ; This node is disabled and will not be called.\nDrag off pins to build functionality.
)

(event EventTick
  (params (DeltaSeconds :type Float%20%28single-precision%29))
  (|CallParentFunction DeltaSeconds))

(fn ConstructionScript
  (|CallParentFunction))

(fn Die
  (params (Position%20Index :type Integer) (ExtraTime :type Float%20%28double-precision%29))
  (|CallParentFunction Position%20Index 0.0)
  (Pawn|UnPossess (Pawn|GetController)))